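; Track tile for a three-lane endless runner that populates itself with random obstacles and pickups.
; On BeginPlay each lane spawns one actor through cascading random rolls: tree, snowcat, barrier, gingerbread, heart or enemy, with coin as fallback.
; When the character overlaps the box, the game mode spawns another tile and the player's walk speed rises slightly within a clamp.
; A Delay on Tick destroys the tile after a fixed lifetime.
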(event `self.ReceiveBeginPlay`
  (`self.SpawnBarriersAndBonuses`))

(event `self.ReceiveTick`
  (params (DeltaSeconds :type "Float (single-precision)"))
  (`KismetSystemLibrary.Delay` 45.0)
  (`self.K2_DestroyActor`))

(event `self.Box.OnComponentBeginOverlap`
  (params (OverlappedComponent :type "PrimitiveComponent Object Reference") (OtherActor :type "Actor Object Reference") (OtherComp :type "PrimitiveComponent Object Reference") (OtherBodyIndex :type Integer) (bFromSweep :type Boolean) (SweepResult :type "HitResult Structure (by ref)"))
  (cast `/Game/Characters/Player/Blueprints/ThirdPersonCharacter` OtherActor)
  (bind _asthird_person_game_mode (cast `/Game/Characters/Player/Blueprints/ThirdPersonGameMode` (`GameplayStatics.GetGameMode`)))
  (`/Game/Characters/Player/Blueprints/ThirdPersonGameMode.SpawnTile` _asthird_person_game_mode)
  ;[1 1 1] Character speed increase
  (bind _asthird_person_character (cast `/Game/Characters/Player/Blueprints/ThirdPersonCharacter` (`GameplayStatics.GetPlayerCharacter` 0)))
  (bind _charactermovement (`Character.CharacterMovement` _asthird_person_character))
  (set `CharacterMovementComponent.MaxWalkSpeed` (`KismetMathLibrary.FClamp` (* (`CharacterMovementComponent.MaxWalkSpeed` _charactermovement) 1.01) 500.0 2000.0) _charactermovement))

(fn `SpawnBarriersAndBonuses`
  (locals (CurrentWorldTransform :type "Transform Structure") (ObstacleIndex :type Integer))
  (`|ExecutionSequence`
    (:`then_0`
      ;[1 1 1] Obstacles generation on first lane
      (`self.SpawnObstaclesOnLane` (`self.FirstLane`)))
    (:`then_1`
      ;[1 1 1] Obstacles generation on second lane
      (`self.SpawnObstaclesOnLane` (`self.SecondLane`)))
    (:`then_2`
      ;[1 1 1] Obstacles generation on third lane
      (`self.SpawnObstaclesOnLane` (`self.ThirdLane`)))))

(fn `SpawnObstacle`
  (params (ActorClass :type "Actor Class Reference") (Lane :type "ArrowComponent Object Reference"))
  (`|SpawnActorFromClass` ActorClass (`SceneComponent.K2_GetComponentToWorld` Lane) "AlwaysSpawn" "OverrideRootScale" null null))

(fn `SpawnObstaclesOnLane`
  (params (Lane :type "ArrowComponent Object Reference"))
  (locals (ObstacleIndex :type Integer))
  (bind _returnvalue (`KismetMathLibrary.RandomFloatInRange` 0.0 2.0))
  (if (`KismetMathLibrary.InRange_FloatFloat` _returnvalue 0.0 0.5)
    (`self.SpawnObstacle` "/Game/Blueprints/Tree_BP.Tree_BP_C" Lane)
    (elif (`KismetMathLibrary.InRange_FloatFloat` _returnvalue 0.4 0.9)
      (`self.SpawnObstacle` "/Game/Blueprints/Snowcat_BP.Snowcat_BP_C" Lane)
      (elif (`KismetMathLibrary.InRange_FloatFloat` _returnvalue 0.8 1.4)
        (`self.SpawnObstacle` "/Game/Blueprints/Barrier_BP.Barrier_BP_C" Lane)
        (elif (`KismetMathLibrary.InRange_FloatFloat` _returnvalue 0.3 0.5)
          (`self.SpawnObstacle` "/Game/Blueprints/Gingerbread_BP.Gingerbread_BP_C" Lane)
          (elif (`KismetMathLibrary.InRange_FloatFloat` _returnvalue 0.2 0.5)
            (`self.SpawnObstacle` "/Game/Blueprints/Heart_BP.Heart_BP_C" Lane)
            (elif (`KismetMathLibrary.InRange_FloatFloat` _returnvalue 0.3 0.6)
              (`self.SpawnObstacle` "/Game/Characters/NPC/Enemy_BP.Enemy_BP_C" Lane)
              (else
                (if (`KismetMathLibrary.InRange_FloatFloat` _returnvalue 0.7)
                  _
                  (else
                    _))
                (`self.SpawnObstacle` "/Game/Blueprints/Coin_BP.Coin_BP_C" Lane)))))))))

(fn `UserConstructionScript`)