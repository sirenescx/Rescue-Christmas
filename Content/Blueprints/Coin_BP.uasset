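; Coin pickup actor that the player character collects by overlapping it.
; On overlap with a ThirdPersonCharacter, it plays a collect sound, increments CoinCounter on the ThirdPersonGameMode and destroys itself.
; An uncollected coin destroys itself after a fixed delay from BeginPlay.
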(event `self.ReceiveBeginPlay`
  (`KismetSystemLibrary.Delay` 45.0)
  (`self.K2_DestroyActor`))

(event `self.ReceiveActorBeginOverlap`
  (params (OtherActor :type "Actor Object Reference"))
  (cast `/Game/Characters/Player/Blueprints/ThirdPersonCharacter` OtherActor)
  (bind _asthird_person_game_mode (cast `/Game/Characters/Player/Blueprints/ThirdPersonGameMode` (`GameplayStatics.GetGameMode`)))
  (`GameplayStatics.PlaySound2D` "/Game/Sound/S_Coin_Collect.S_Coin_Collect" 1.0 1.0 0.0 null null)
  (bind _result (`/Engine/EditorBlueprintResources/StandardMacros.IncrementInt` (`/Game/Characters/Player/Blueprints/ThirdPersonGameMode.CoinCounter` _asthird_person_game_mode))
    (:`  `
      (set `/Game/Characters/Player/Blueprints/ThirdPersonGameMode.CoinCounter` _result _asthird_person_game_mode)
      (`self.K2_DestroyActor`))))

(fn `UserConstructionScript`)