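; First_Tile_BP is a track tile for what appears to be a three-lane runner, destroying itself through a 45-second Delay on Tick.
; SpawnBarriersAndBonuses, not called within this graph, spawns one actor at each lane component's transform.
; SpawnObstaclesOnLane picks barriers, a ramp, gingerbread, life or enemy through chained range checks, each on a fresh random roll.
; Coin is the fallback, as both branches of the last check spawn it.
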(event `self.ReceiveTick`
  (params (DeltaSeconds :type "Float (single-precision)"))
  (`KismetSystemLibrary.Delay` 45.0)
  (`self.K2_DestroyActor`))

(fn `SpawnBarriersAndBonuses`
  (locals (CurrentWorldTransform :type "Transform Structure") (ObstacleIndex :type Integer))
  (`|ExecutionSequence`
    (:`then_0`
      ;[1 1 1] Obstacles generation on first lane
      (`self.SpawnObstaclesOnLane` (`self.FirstLane`)))
    (:`then_1`
      ;[1 1 1] Obstacles generation on second lane
      (`self.SpawnObstaclesOnLane` (`self.SecondLane`)))
    (:`then_2`
      ;[1 1 1] Obstacles generation on third lane
      (`self.SpawnObstaclesOnLane` (`self.ThirdLane`)))))

(fn `SpawnObstacle`
  (params (ActorClass :type "Actor Class Reference") (Lane :type "ArrowComponent Object Reference"))
  (`|SpawnActorFromClass` ActorClass (`SceneComponent.K2_GetComponentToWorld` Lane) "AlwaysSpawn" "OverrideRootScale" null null))

(fn `SpawnObstaclesOnLane`
  (params (Lane :type "ArrowComponent Object Reference"))
  (locals (ObstacleIndex :type Integer))
  (bind _returnvalue (`KismetMathLibrary.RandomFloatInRange` 0.0 2.0))
  (if (`KismetMathLibrary.InRange_FloatFloat` _returnvalue 0.0 0.5)
    (`self.SpawnObstacle` "/Game/Blueprints/SecondBarrier_BP.SecondBarrier_BP_C" Lane)
    (elif (`KismetMathLibrary.InRange_FloatFloat` _returnvalue 0.4 0.9)
      (`self.SpawnObstacle` "/Game/Blueprints/Ramp_BP.Ramp_BP_C" Lane)
      (elif (`KismetMathLibrary.InRange_FloatFloat` _returnvalue 0.8 1.4)
        (`self.SpawnObstacle` "/Game/Blueprints/Barrier_BP.Barrier_BP_C" Lane)
        (elif (`KismetMathLibrary.InRange_FloatFloat` _returnvalue 0.3 0.5)
          (`self.SpawnObstacle` "/Game/Blueprints/Gingerbread_BP.Gingerbread_BP_C" Lane)
          (elif (`KismetMathLibrary.InRange_FloatFloat` _returnvalue 0.2 0.5)
            (`self.SpawnObstacle` "/Game/Blueprints/Life_BP.Life_BP_C" Lane)
            (elif (`KismetMathLibrary.InRange_FloatFloat` _returnvalue 0.3 0.6)
              (`self.SpawnObstacle` "/Game/Characters/NPC/Enemy_BP.Enemy_BP_C" Lane)
              (else
                (if (`KismetMathLibrary.InRange_FloatFloat` _returnvalue 0.7)
                  _
                  (else
                    _))
                (`self.SpawnObstacle` "/Game/Blueprints/Coin_BP.Coin_BP_C" Lane)))))))))

(fn `UserConstructionScript`)