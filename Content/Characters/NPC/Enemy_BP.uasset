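; Enemy NPC that acts as a moving hazard, damaging the third-person character when it overlaps them.
; A timeline starts on BeginPlay and each update adds its track value to the static mesh's world Y position, without sweeping.
; On actor overlap, it casts to ThirdPersonCharacter and calls that character's TakeDamage with a fixed amount, passing itself as the obstacle.
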(event `self.ReceiveBeginPlay`
  (bind _staticmesh (`self.StaticMesh`))
  (bind (_direction _movement_track) (`Timeline|Continious_Movement_Timeline`)
    (:`Update`
      (`SceneComponent.K2_SetWorldLocation` _staticmesh (+ (`SceneComponent.K2_GetComponentLocation` _staticmesh) (`KismetMathLibrary.MakeVector` 0.0 _movement_track)) false false))))

(event `self.ReceiveActorBeginOverlap`
  (params (OtherActor :type "Actor Object Reference"))
  (bind _asthird_person_character (cast `/Game/Characters/Player/Blueprints/ThirdPersonCharacter` OtherActor))
  (bind _asthird_person_character_2 (cast `/Game/Characters/Player/Blueprints/ThirdPersonCharacter` _asthird_person_character))
  (`/Game/Characters/Player/Blueprints/ThirdPersonCharacter.TakeDamage` _asthird_person_character_2 (`KismetMathLibrary.FTrunc` 50.0) self))

(fn `UserConstructionScript`)