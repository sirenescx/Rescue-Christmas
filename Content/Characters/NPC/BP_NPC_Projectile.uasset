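; BP_NPC_Projectile is an NPC projectile that flies straight and damages the player's ThirdPersonCharacter.
; Tick moves it along its forward vector by Speed times delta time, without sweep or a movement component.
; A Sphere overlap casts to ThirdPersonCharacter and calls its TakeDamage with a fixed amount, passing itself as the obstacle.
; The projectile does not destroy itself on hit or after a lifetime in this graph.
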(event `self.ReceiveTick`
  (params (DeltaSeconds :type "Float (single-precision)"))
  (`self.K2_SetActorLocation` (+ (`self.K2_GetActorLocation`) (* (* (`self.GetActorForwardVector`) (`self.Speed`)) DeltaSeconds))))

(event `self.ReceiveActorBeginOverlap`
  (params (OtherActor :type "Actor Object Reference")))

(event `self.Sphere.OnComponentBeginOverlap`
  (params (OverlappedComponent :type "PrimitiveComponent Object Reference") (OtherActor :type "Actor Object Reference") (OtherComp :type "PrimitiveComponent Object Reference") (OtherBodyIndex :type Integer) (bFromSweep :type Boolean) (SweepResult :type "HitResult Structure (by ref)"))
  (bind _asthird_person_character (cast `/Game/Characters/Player/Blueprints/ThirdPersonCharacter` OtherActor))
  (`/Game/Characters/Player/Blueprints/ThirdPersonCharacter.TakeDamage` _asthird_person_character (`KismetMathLibrary.FTrunc` 50.0) self))

(fn `UserConstructionScript`)